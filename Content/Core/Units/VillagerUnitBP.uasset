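; Villager unit with a modular appearance driven by its profession, built from base body, hair, beard, clothes and tool meshes.
; The construction script makes the parts follow the body's pose via master pose, and BeginPlay passes idle and walk/run animations to VillagerAnim.
; SetupClothing picks outfit type by profession, randomizing hair and beard except for Unassigned villagers.
; ApplyClothing then swaps meshes and materials, setting profession colors and tools.
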(event `self.ReceiveBeginPlay`
  (bind _asvillager_anim (cast `/Game/Models/Villagers/Final/VillagerAnim` (`SkeletalMeshComponent.GetAnimInstance` (`self.BaseMesh`))))
  (set `/Game/Models/Villagers/Final/VillagerAnim.IdleSequence` (`self.IdleAnimation`) _asvillager_anim)
  (set `/Game/Models/Villagers/Final/VillagerAnim.RunWalkSequence` (`self.WalkRunAnimation`) _asvillager_anim)
  (set `/Game/Models/Villagers/Final/VillagerAnim.RunWalkSequenceAdvanced` (`self.WalkRunAnimationAdvanced`) _asvillager_anim))

(fn `ApplyClothing`
  ;[1 1 1] Hair
  (switch `int` (`self.HairNum`)
    (:`0`
      _)
    (:`1`
      (`SkinnedMeshComponent.SetSkinnedAssetAndUpdate` (`self.MeshHair`) "/Game/Models/Villagers/Final/Addon/Hair/FinalHairAlt1.FinalHairAlt1" true))
    (:`2`
      (`SkinnedMeshComponent.SetSkinnedAssetAndUpdate` (`self.MeshHair`) "/Game/Models/Villagers/Final/Addon/Hair/FinalHairAlt2.FinalHairAlt2" true))
    (:`3`
      (`SkinnedMeshComponent.SetSkinnedAssetAndUpdate` (`self.MeshHair`) "/Game/Models/Villagers/Final/Addon/Hair/FinalHairAlt3.FinalHairAlt3" true))
    (:`4`
      (`SkinnedMeshComponent.SetSkinnedAssetAndUpdate` (`self.MeshHair`) "/Game/Models/Villagers/Final/Addon/Hair/FinalHairAlt4.FinalHairAlt4" true))
    (:`5`
      (`SkinnedMeshComponent.SetSkinnedAssetAndUpdate` (`self.MeshHair`) "/Game/Models/Villagers/Final/Addon/Hair/FinalHairAlt5.FinalHairAlt5" true)))
  (switch `int` (`self.HairColor`)
    (:`0`
      _)
    (:`1`
      (`PrimitiveComponent.SetMaterial` (`self.MeshHair`) 0 "/Game/Models/Materials/Villager/VHairBlonde.VHairBlonde")
      (`PrimitiveComponent.SetMaterial` (`self.MeshBeard`) 0 "/Game/Models/Materials/Villager/VHairBlonde.VHairBlonde")
      (`PrimitiveComponent.SetMaterial` (`self.BaseMesh`) 1 "/Game/Models/Materials/Villager/VHairBlonde.VHairBlonde"))
    (:`2`
      (`PrimitiveComponent.SetMaterial` (`self.MeshHair`) 0 "/Game/Models/Materials/Villager/VHairGinger.VHairGinger")
      (`PrimitiveComponent.SetMaterial` (`self.MeshBeard`) 0 "/Game/Models/Materials/Villager/VHairGinger.VHairGinger")
      (`PrimitiveComponent.SetMaterial` (`self.BaseMesh`) 1 "/Game/Models/Materials/Villager/VHairGinger.VHairGinger"))
    (:`3`
      (`PrimitiveComponent.SetMaterial` (`self.MeshHair`) 0 "/Game/Models/Materials/Villager/VHairBrownLight.VHairBrownLight")
      (`PrimitiveComponent.SetMaterial` (`self.MeshBeard`) 0 "/Game/Models/Materials/Villager/VHairBrownLight.VHairBrownLight")
      (`PrimitiveComponent.SetMaterial` (`self.BaseMesh`) 1 "/Game/Models/Materials/Villager/VHairBrownLight.VHairBrownLight"))
    (:`4`
      (`PrimitiveComponent.SetMaterial` (`self.MeshHair`) 0 "/Game/Models/Materials/Villager/VHairBrownDark.VHairBrownDark")
      (`PrimitiveComponent.SetMaterial` (`self.MeshBeard`) 0 "/Game/Models/Materials/Villager/VHairBrownDark.VHairBrownDark")
      (`PrimitiveComponent.SetMaterial` (`self.BaseMesh`) 1 "/Game/Models/Materials/Villager/VHairBrownDark.VHairBrownDark")))
  ;[1 1 1] Beard
  (switch `int` (`self.BeardNum`)
    (:`0`
      _)
    (:`1`
      (`SkinnedMeshComponent.SetSkinnedAssetAndUpdate` (`self.MeshBeard`) "/Game/Models/Villagers/Final/Addon/Beard/FinalBeardAlt1.FinalBeardAlt1" true)))
  ;[1 1 1] Clothing
  (switch `int` (`self.ClothesNum`)
    (:`1`
      (`SkinnedMeshComponent.SetSkinnedAssetAndUpdate` (`self.MeshClothes`) "/Game/Models/Villagers/Final/Addon/Clothing/FinalClothesAlt1.FinalClothesAlt1" true)
      (`SkinnedMeshComponent.SetSkinnedAssetAndUpdate` (`self.BaseMesh`) "/Game/Models/Villagers/Final/VillagerModelBaseCut1.VillagerModelBaseCut1" true))
    (:`2`
      (`SkinnedMeshComponent.SetSkinnedAssetAndUpdate` (`self.MeshClothes`) "/Game/Models/Villagers/Final/Addon/Clothing/FinalClothesAlt2.FinalClothesAlt2" true)
      (`SkinnedMeshComponent.SetSkinnedAssetAndUpdate` (`self.BaseMesh`) "/Game/Models/Villagers/Final/VillagerModelBaseCut2.VillagerModelBaseCut2" true)))
  (`|ExecutionSequence`
    (:`then_0`
      (bind _returnvalue (`ProfessionComponent.GetVillagerClass` (`self.Profession`)))
      (`KismetSystemLibrary.PrintString` (`|GetEnumeratorNameAsString` _returnvalue))
      (switch `EEndlingClass` _returnvalue
        (:`Unassigned`
          (`PrimitiveComponent.SetMaterial` (`self.BaseMesh`) 2 "/Game/Models/Materials/Villager/VSkin.VSkin")
          (`PrimitiveComponent.SetMaterial` (`self.MeshClothes`) 1 "/Game/Models/Materials/Villager/VTunicRed.VTunicRed")
          (`PrimitiveComponent.SetMaterial` (`self.MeshClothes`) 0 "/Game/Models/Materials/Villager/VTunicLightColor.VTunicLightColor"))
        (:`Lumberjack`
          (`SkinnedMeshComponent.SetSkinnedAssetAndUpdate` (`self.MeshTool`) "/Game/Models/Villagers/Final/Addon/Tools/FinalToolAxe.FinalToolAxe" true)
          (`PrimitiveComponent.SetMaterial` (`self.BaseMesh`) 2 "/Game/Models/Materials/Villager/VTunicBlue.VTunicBlue")
          (`PrimitiveComponent.SetMaterial` (`self.MeshClothes`) 1 "/Game/Models/Materials/Villager/VTunicClassic.VTunicClassic")
          (`PrimitiveComponent.SetMaterial` (`self.MeshClothes`) 0 "/Game/Models/Materials/Villager/VHairBrown.VHairBrown"))
        (:`Miner`
          (`PrimitiveComponent.SetMaterial` (`self.MeshClothes`) 1 "/Game/Models/Materials/Villager/VTunicWhite.VTunicWhite")
          (`PrimitiveComponent.SetMaterial` (`self.BaseMesh`) 2 "/Game/Models/Materials/Villager/VTunicGrey.VTunicGrey")
          (`SkinnedMeshComponent.SetSkinnedAssetAndUpdate` (`self.MeshTool`) "/Game/Models/Villagers/Final/Addon/Tools/FinalToolPick.FinalToolPick" true)
          (`PrimitiveComponent.SetMaterial` (`self.MeshClothes`) 0 "/Game/Models/Materials/Villager/VHairBrown.VHairBrown" :!label _label))
        (:`Gatherer`
          (`PrimitiveComponent.SetMaterial` (`self.MeshClothes`) 1 "/Game/Models/Materials/Villager/VTunicRed.VTunicRed")
          (`PrimitiveComponent.SetMaterial` (`self.BaseMesh`) 2 "/Game/Models/Materials/Villager/VTunicGreenDark.VTunicGreenDark")
          (goto _label))
        (:`Woodworker`
          (`PrimitiveComponent.SetMaterial` (`self.MeshClothes`) 2 "/Game/Models/Materials/Villager/VTunicGreenMed.VTunicGreenMed")
          (`PrimitiveComponent.SetMaterial` (`self.BaseMesh`) 2 "/Game/Models/Materials/Villager/VTunicOrange.VTunicOrange")
          (`PrimitiveComponent.SetMaterial` (`self.MeshClothes`) 0 "/Game/Models/Materials/Villager/VTunicWhite.VTunicWhite" :!label _label_2)
          (`PrimitiveComponent.SetMaterial` (`self.MeshClothes`) 1 "/Game/Models/Materials/Villager/VHairBrown.VHairBrown")
          (`SkinnedMeshComponent.SetSkinnedAssetAndUpdate` (`self.MeshTool`) null true))
        (:`Stonemason`
          (`PrimitiveComponent.SetMaterial` (`self.MeshClothes`) 2 "/Game/Models/Materials/Villager/VTunicBrown.VTunicBrown")
          (`PrimitiveComponent.SetMaterial` (`self.BaseMesh`) 2 "/Game/Models/Materials/Villager/VTunicWhite.VTunicWhite")
          (goto _label_2))
        (:`Cook`
          (`PrimitiveComponent.SetMaterial` (`self.MeshClothes`) 2 "/Game/Models/Materials/Villager/VTunicBlue.VTunicBlue")
          (`PrimitiveComponent.SetMaterial` (`self.BaseMesh`) 2 "/Game/Models/Materials/Villager/VTunicRed.VTunicRed")
          (goto _label_2))))))

(fn `SetupClothing`
  (bind _returnvalue (`KismetMathLibrary.RandomIntegerInRange` 0 4))
  (bind _returnvalue_2 (`ProfessionComponent.GetVillagerClass` (`self.Profession`)))
  (switch `EEndlingClass` _returnvalue_2
    (:`Unassigned`
      (set `self.ClothesNum` 1)
      (set `self.HairNum` 4)
      (set `self.BeardNum` 1)
      (set `self.HairColor` 0))
    (:`Lumberjack`
      (set `self.ClothesNum` 1 :!label _label)
      (set `self.HairNum` (`KismetMathLibrary.RandomIntegerInRange` 0 5) :!label _label_2)
      (set `self.BeardNum` (`KismetMathLibrary.RandomIntegerInRange` 0 1))
      (set `self.HairColor` _returnvalue)
      (if (!= _returnvalue 2)
        _
        (elif (== (`KismetMathLibrary.RandomIntegerInRange` 0 1) 0)
          (set `self.HairColor` 0)
          (else
            (set `self.HairColor` 2)))))
    (:`Miner`
      (goto _label))
    (:`Gatherer`
      (goto _label))
    (:`Woodworker`
      (set `self.ClothesNum` 2 :!label _label_3)
      (goto _label_2))
    (:`Stonemason`
      (goto _label_3))
    (:`Cook`
      (goto _label_3)))
  (`self.ApplyClothing`))

(fn `UserConstructionScript`
  (bind _basemesh (`self.BaseMesh`))
  (`SkinnedMeshComponent.SetLeaderPoseComponent` (`self.MeshHair`) _basemesh false)
  (`SkinnedMeshComponent.SetLeaderPoseComponent` (`self.MeshBeard`) _basemesh false)
  (`SkinnedMeshComponent.SetLeaderPoseComponent` (`self.MeshClothes`) _basemesh false)
  (`SkinnedMeshComponent.SetLeaderPoseComponent` (`self.MeshTool`) _basemesh false))