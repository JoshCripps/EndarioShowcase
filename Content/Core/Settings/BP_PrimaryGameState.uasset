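; BP_PrimaryGameState is a game state Blueprint that runs the in-game clock and calendar.
; BeginPlay builds a DateTime struct from the year-to-second variables.
; Each Tick, CalculateTime advances game time and the day counter using delta time and game speed, then SetClockCalendar runs.
; Tick also prints the struct's seconds, and an unconnected SetDateTime call never runs.
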(event `self.ReceiveBeginPlay`
  (set `self.DateTimeStruct` (`KismetMathLibrary.MakeDateTime` (`self.Years`) (`self.Months`) (`self.Days`) (`self.Hours`) (`self.Minutes`) (`self.Seconds`))))

(event `self.ReceiveTick`
  (params (DeltaSeconds :type "Float (single-precision)"))
  (bind (_gametimeout _daycounterout) (`self.CalculateTime` DeltaSeconds (`self.GameSpeed`) (`self.GameTime`)))
  (set `self.GameTime` _gametimeout)
  (set `self.DayCounter` _daycounterout)
  (`self.SetClockCalendar`)
  (`KismetSystemLibrary.PrintString` (`KismetStringLibrary.Conv_IntToString` (`.Second` (`KismetMathLibrary.BreakDateTime` (`self.DateTimeStruct`))))))

(fn `UserConstructionScript`)